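; BP_Balle is a projectile actor with an animated skeletal mesh that reacts to impact, flops when it stops, then removes itself.
; On bounce, it sets gravity scale to normal, starts a sped-up impact montage and immediately zeroes bounciness so the projectile loses its rebound.
; When projectile movement stops, it plays a flopping montage and destroys the actor once that montage completes or is interrupted.
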(event OnProjectileBounce(ProjectileMovement)
  (params (ImpactResult :type Hit%20Result%20Structure%20%28by%20ref%29) (ImpactVelocity :type Vector%20%28by%20ref%29 :default "0, 0, 0"))
  (bind _projectilemovement (Variables|Default|GetProjectileMovement))
  (Variables|/Script/Engine.ProjectileMovementComponent|SetProjectileGravityScale _projectilemovement 1.0)
  (Animation|Montage|PlayMontage (Variables|Default|GetSkeletalMesh) "/Game/Animation/ImpactAnim_Montage.ImpactAnim_Montage" 2.0
    (:then
      (Variables|/Script/Engine.ProjectileMovementComponent|SetBounciness _projectilemovement 0.0))))

(event OnProjectileStop(ProjectileMovement)
  (params (ImpactResult :type Hit%20Result%20Structure%20%28by%20ref%29))
  (Animation|Montage|PlayMontage (Variables|Default|GetSkeletalMesh) "/Game/Animation/FloppingAnim_Montage.FloppingAnim_Montage"
    (:OnCompleted
      _)
    (:OnInterrupted
      _))
  (Actor|DestroyActor))

(event EventBeginPlay)

(event Collision|EventActorBeginOverlap
  (params (OtherActor :type Actor%20Object%20Reference)))

(event EventTick
  (params (DeltaSeconds :type Float%20%28single-precision%29)))

(fn ConstructionScript)